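; Rock projectile, filed under big_guy, that launches at the player and damages them on a fast hit.
; On BeginPlay it impulses its Sphere toward the player pawn and sets a five-second lifespan.
; Tick applies a single second homing impulse once it comes within range of the player.
; A hit on a player-tagged actor at high enough Sphere speed calls Damage once and destroys the rock.
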(event EventBeginPlay
  (bind _sphere (Variables|Default|GetSphere))
  (bind _returnvalue (Actor|GetActorOfClass "/Game/Blueprints/character/player_character.player_character_C"))
  (Variables|Default|SetplayerC _returnvalue)
  (Actor|SetLifeSpan 5.0)
  (Physics|AddImpulse _sphere (* (Math|Vector|Normalize (- (Transformation|GetActorLocation (Game|Player|GetPlayerPawn 0)) (Transformation|GetWorldLocation _sphere))) (Variables|Default|GetthrowStrength)) "None" true))

(event EventTick
  (params (DeltaSeconds :type Float%20%28single-precision%29))
  (bind _sphere (Variables|Default|GetSphere))
  (if (<= (Math|Vector|Distance(Vector) (Transformation|GetActorLocation (Variables|Default|GetplayerC)) (Transformation|GetWorldLocation (Variables|Default|GetSphere))) 5e+03)
    (Utilities|FlowControl|DoOnce false
      (:Completed
        (Physics|AddImpulse _sphere (* (Math|Vector|Normalize (- (Transformation|GetActorLocation (Game|Player|GetPlayerPawn 0)) (Transformation|GetWorldLocation _sphere))) (Variables|Default|GetsecondImpulseStr)) "None" true)))))

(event Collision|EventHit
  (params (MyComp :type Primitive%20Component%20Object%20Reference) (Other :type Actor%20Object%20Reference) (OtherComp :type Primitive%20Component%20Object%20Reference) (bSelfMoved :type Boolean) (HitLocation :type Vector :default "0, 0, 0") (HitNormal :type Vector :default "0, 0, 0") (NormalImpulse :type Vector :default "0, 0, 0") (Hit :type Hit%20Result%20Structure%20%28by%20ref%29))
  (if (Utilities|IsValid Other)
    (if (Actor|ActorHasTag Other "player")
      (bind _returnvalue (Actor|GetActorOfClass "/Game/Blueprints/character/player_character.player_character_C"))
      (if (>= (Math|Vector|VectorLength (Transformation|GetComponentVelocity (Variables|Default|GetSphere))) 2e+03)
        (Utilities|FlowControl|DoOnce false
          (:Completed
            (Default|Damage _returnvalue)
            (Actor|DestroyActor)))))))

(fn ConstructionScript)
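; A timer actor that measures how long passes between a player leaving a start box and a pawn reaching an end box.
; Tick polls both boxes, checking only the first overlapping pawn: while one tagged player is in Box, it keeps refreshing the start time and resetting a DoOnce.
; Otherwise, any pawn in Box1 fires that DoOnce, which computes the elapsed time and prints it once per reset.
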(event EventBeginPlay)

(event Collision|EventActorBeginOverlap
  (params (OtherActor :type Actor%20Object%20Reference)))

(event EventTick
  (params (DeltaSeconds :type Float%20%28single-precision%29))
  (bind _box (Variables|Default|GetBox))
  (bind _overlappingactors (Collision|GetOverlappingActors _box "/Script/Engine.Pawn" :!class /Script/Engine.PrimitiveComponent))
  (bind _output (Utilities|Array|Get(acopy) _overlappingactors))
  (if (Utilities|IsValid _output)
    (if (Actor|ActorHasTag _output "player")
      (Variables|Default|SettimerStart (Utilities|Time|GetTimeSeconds))
      (goto _label Reset)
      (else
        _)))
  (if (Utilities|IsValid (Utilities|Array|Get(acopy) (Collision|GetOverlappingActors (Variables|Default|GetBox1) "/Script/Engine.Pawn" :!class /Script/Engine.PrimitiveComponent)))
    (Utilities|FlowControl|DoOnce false :!label _label
      (:Completed
        (Variables|Default|SetendTime (- (Utilities|Time|GetTimeSeconds) (Variables|Default|GettimerStart)))
        (Development|PrintString (Utilities|String|ToString(Float) (Variables|Default|GetendTime)))))))

(fn ConstructionScript)
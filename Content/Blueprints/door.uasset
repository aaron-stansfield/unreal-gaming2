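; Interactable swing door that opens 80 degrees away from the player's side and returns to zero yaw on the next interact.
; Tick sets presence from actor overlaps, using OutsideColl and a "player" tag to pick the swing side.
; Interact sets the target and opens a Gate, letting LiveLink update events drive OpenDoor.
; OpenDoor steps yaw by a fixed, frame-rate-independent-less increment until truncated angles match, storing direction for closing.
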(event OnLiveLinkUpdated(LiveLinkComponentController)
  (params (DeltaTime :type Float%20%28single-precision%29))
  (bind _closegate (Variables|Default|GetcloseGate))
  ;[0.3365 0.143 1 1 27] moving door :(
  (if (not (Variables|Default|Getdoor%20open))
    (if _closegate
      (goto _label Close)
      (else
        (Utilities|FlowControl|Gate true :!label _label
          (:Exit
            (CallFunction|OpenDoor false)))))
    (elif _closegate
      (goto _label_2 Close)
      (else
        (Utilities|FlowControl|Gate false :!label _label_2
          (:Exit
            (CallFunction|OpenDoor false)))))))

(event Input|EnhancedActionEvents|EnhancedInputActioninteract
  (params (ActionValue :type Boolean) (ElapsedSeconds :type Float%20%28double-precision%29) (TriggeredSeconds :type Float%20%28double-precision%29) (InputAction :type Input%20Action%20Object%20Reference :default "/Game/Blueprints/character/interact.interact"))
  (bind _staticmesh (Variables|Actor|GetStaticMesh))
  (bind _relativerotation (Variables|/Script/Engine.SceneComponent|GetRelativeRotation _staticmesh))
  ;[0.3365 0.143 1 1 27] moving door :(
  (if (not (Variables|Default|Getopening))
    (if (Variables|Default|Getdoor%20open)
      (Variables|Default|SetcloseGate false)
      (Variables|Default|SetdoorTarget 0.0)
      (if (Variables|Default|GetcloseGate)
        (Utilities|FlowControl|Gate false) ; enters at Close
        (else
          (Utilities|FlowControl|Gate false) ; enters at Open
        ))
      (else
        (Variables|Default|SetcloseGate false)
        (if (Variables|Default|Getpresence)
          (if (Variables|Default|Getoutside%20presence)
            (Variables|Default|SetdoorTarget (+ (.yaw _relativerotation) -8e+01))
            (else
              (Variables|Default|SetdoorTarget (+ (.yaw _relativerotation) 8e+01))))
          (if (Variables|Default|GetcloseGate)
            (Utilities|FlowControl|Gate true) ; enters at Close
            (else
              (Utilities|FlowControl|Gate true) ; enters at Open
            )))))))

(event EventTick
  (params (DeltaSeconds :type Float%20%28single-precision%29))
  (bind _outside_coll (Variables|Collision|Getoutside%20coll))
  (bind _overlappingactors (Collision|GetOverlappingActors _outside_coll "/Script/Engine.Character" :!class /Script/Engine.PrimitiveComponent))
  (bind _output (Utilities|Array|Get(acopy) _overlappingactors))
  (bind _returnvalue (Utilities|IsValid _output))
  ;[1 0.1245 0.1706 1 27] check presence
  (Variables|Default|SetDelta%20Seconds DeltaSeconds)
  (if _returnvalue
    (Variables|Default|Setoutside%20presence (Actor|ActorHasTag _output "player"))
    (else
      (Variables|Default|Setoutside%20presence _returnvalue)))
  (if (Utilities|IsValid (Utilities|Array|Get(acopy) (Collision|GetOverlappingActors (Components|GetOwner (Variables|Actor|GetStaticMesh)) 0 :!class /Script/Engine.Actor)))
    (Variables|Default|Setpresence true)
    (else
      (Variables|Default|Setpresence false))))

(event EventBeginPlay
  ;[0.004728 0.4747 1 1 27] startup & enabling input
  (Variables|Default|Setdoor%20open false)
  (Variables|Default|Setoutside%20presence false)
  (Input|EnableInput (Game|GetPlayerController 0)))

(fn ConstructionScript)

(fn OpenDoor
  (params (NewParam :type Boolean))
  (bind _staticmesh (Variables|Actor|GetStaticMesh))
  (bind _relativerotation (Variables|/Script/Engine.SceneComponent|GetRelativeRotation _staticmesh))
  (Variables|Default|Setopening true)
  (LocalVariables|SetdoorRot (.yaw (Variables|/Script/Engine.SceneComponent|GetRelativeRotation (Variables|Actor|GetStaticMesh))))
  (if (not (Variables|Default|GetcloseGate))
    (Math|Float|CompareFloat 0.0 (Variables|Default|GetdoorTarget)
      (:>
        (LocalVariables|SetdirectionToOpen -2.0 :!label _label))
      (:==
        (if (Utilities|String|Contains (Variables|Default|GetopenDir) "inward")
          (LocalVariables|SetdirectionToOpen 2.0 :!label _label_2)
          (else
            (goto _label))))
      (:<
        (goto _label_2)))
    (bind _output_get (LocalVariables|SetdoorRot (.yaw _relativerotation)))
    (Transformation|SetRelativeRotation (Variables|Actor|GetStaticMesh) (Math|Interpolation|RInterpTo (Math|Rotator|MakeRotator 0.0 0.0 _output_get) (Math|Rotator|MakeRotator 0.0 0.0 (+ (.yaw _relativerotation) (LocalVariables|GetdirectionToOpen))) 1.0 1.0) false false)
    (bind _output_get_2 (LocalVariables|SetdoorRot (.yaw (Variables|/Script/Engine.SceneComponent|GetRelativeRotation (Variables|Actor|GetStaticMesh)))))
    (Math|Integer|CompareInt (Math|Float|Truncate _output_get_2) (Math|Float|Truncate (Variables|Default|GetdoorTarget))
      (:==
        (Math|Float|CompareFloat 0.0 (Variables|Default|GetdoorTarget)
          (:>
            (Variables|Default|SetopenDir "inwards")
            (Variables|Default|Setdoor%20open true :!label _label_3))
          (:==
            (Variables|Default|Setdoor%20open false))
          (:<
            (Variables|Default|SetopenDir "our")
            (goto _label_3)))
        (Variables|Default|SetcloseGate true)
        (Variables|Default|Setopening false)))))
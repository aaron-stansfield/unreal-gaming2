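; First-person player character with parkour movement (wallrun, wall jump, grapple, mantle, slide), health, and item pickup, drop and attack.
; Tick alternates via FlipFlop between tag-filtered wall traces and grapple/mantle traces, setting state for jump and grapple inputs and crosshair colours.
; Timelines drive camera effects and grapple impulses; health and inventory update UiBlueprint, and death opens the menu level.
; Sprint is disconnected, leaving the sprint-gated slide without its trigger.
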(event OnLiveLinkUpdated(LiveLinkComponentController)
  (params (DeltaTime :type Float%20%28single-precision%29))
  (bind _returnvalue (Game|Player|GetPlayerPawn 0))
  (bind _returnvalue_2 (Transformation|GetVelocity _returnvalue))
  ;[1 1 1] speed control (pls find another way)
  (Variables|/Script/Engine.CharacterMovementComponent|SetGroundFriction (Variables|Character|GetCharacterMovement) (Math|Float|Lerp 8.0 0.1 (Math|Float|NormalizetoRange (+ (Math|Float|Absolute(Float) (.x _returnvalue_2)) (Math|Float|Absolute(Float) (.y _returnvalue_2))) 1.3e+03 4e+03))))

(event Custom|damage
  (bind _returnvalue (Game|GetPlayerController 0))
  ;[1 1 1] damage
  (Math|Integer|CompareInt (Variables|Default|Gethealth)
    (:>
      (bind _foundwidgets (Widget|GetAllWidgetsOfClass "/Game/Blueprints/character/uiBlueprint.uiBlueprint_C" true))
      (bind _result (Math|Integer|DecrementInt (Variables|Default|Gethealth))
        (:%20%20
          (bind _output_get (Variables|Default|Sethealth _result))
          (Class|Throbber|SetNumberOfPieces (Variables|/Game/Blueprints/character/uiBlueprint.uiBlueprint_C|GetThrobber_0 (Utilities|Array|Get(acopy) _foundwidgets)) _output_get)
          (bind _newtrack_0 (Timeline|Timeline_6 PlayFromStart)
            (:Update
              (Class|BackgroundBlur|SetBlurStrength (Variables|/Game/Blueprints/character/uiBlueprint.uiBlueprint_C|GetBackgroundBlur_124 (Utilities|Array|Get(acopy) _foundwidgets)) (Math|Float|NormalizetoRange _newtrack_0 0.0 8.0))
              (Camera|SetFieldOfView (Variables|Default|GetCamera) (+ (Variables|Default|GetcameraFov) (* _newtrack_0 3.0))))))))
    (:==
      (Widget|RemovefromParent (Variables|Default|GetcrosshairReference) :!label _label)
      (Game|OpenLevel(byName) "menu")
      (Variables|/Script/Engine.PlayerController|SetbShowMouseCursor _returnvalue true)
      (Input|SetInputModeUIOnly _returnvalue 0 "DoNotLock" false))
    (:<
      (goto _label))))

(event Custom|noise
  (bind _returnvalue (Game|Player|GetPlayerPawn 0))
  ;[1 1 1] makin shnoises
  (Class|AISenseHearing|ReportNoiseEvent (Transformation|GetActorLocation _returnvalue) 1.0 _returnvalue 0.0 "None")
  (Utilities|FlowControl|Delay 3.0))

(event Input|EnhancedActionEvents|EnhancedInputActionpickUp
  (params (ActionValue :type Boolean) (ElapsedSeconds :type Float%20%28double-precision%29) (TriggeredSeconds :type Float%20%28double-precision%29) (InputAction :type Input%20Action%20Object%20Reference :default "/Game/Blueprints/character/pickUp.pickUp"))
  ;[1 1 1] pick up
  (CallFunction|PickUp))

(event Input|EnhancedActionEvents|EnhancedInputActionjump
  (params (ActionValue :type Boolean) (ElapsedSeconds :type Float%20%28double-precision%29) (TriggeredSeconds :type Float%20%28double-precision%29) (InputAction :type Input%20Action%20Object%20Reference :default "/Game/Blueprints/character/jump.jump"))
  (bind _returnvalue (Game|GetPlayerCharacter 0))
  (bind _camera (Variables|Default|GetCamera))
  (bind _walljumpamount (Variables|Default|GetwallJumpAmount))
  (bind _returnvalue_2 (Math|Vector|GetRightVector _camera))
  (bind _returnvalue_3 (Transformation|GetVelocity _returnvalue))
  ;[1 1 1] jumpy
  (:Triggered
    ;;[1 1 1] mantle
    (if (Variables|Default|GetcanMantle) :!label _label
      (Utilities|FlowControl|DoOnce false :!label _label_2
        (:Completed
          (Variables|/Script/Engine.MovementComponent|SetVelocity (Variables|/Script/Engine.Character|GetCharacterMovement _returnvalue) (Math|Vector|MakeVector (.x _returnvalue_3) (.y _returnvalue_3) 8e+02))
          (Utilities|FlowControl|Delay 1.0)
          (goto _label_2 Reset)))))
  (:Started
    (if (Variables|Default|GetisWallrunning)
      (if (Variables|Default|GetwallSide)
        (Variables|Default|SetWallJumpSideVel (Math|Vector|NegateVector _returnvalue_2))
        (else
          (Variables|Default|SetWallJumpSideVel _returnvalue_2)))
      (Character|LaunchCharacter _returnvalue (+ (* (Variables|Default|GetWallJumpSideVel) _walljumpamount) (* (Math|Vector|GetUpVector _camera) (* _walljumpamount 2.0)) (Math|Vector|GetForwardVector _camera)) false true)
      (else
        (Character|Jump))))
  (:Ongoing
    (goto _label))
  (:Completed
    (Character|StopJumping)))

(event Input|EnhancedActionEvents|EnhancedInputActioninteract
  (params (ActionValue :type Boolean) (ElapsedSeconds :type Float%20%28double-precision%29) (TriggeredSeconds :type Float%20%28double-precision%29) (InputAction :type Input%20Action%20Object%20Reference :default "/Game/Blueprints/character/interact.interact"))
  ;[1 1 1] Interacty
  (bind _outactors (Actor|GetAllActorsOfClass "/Game/Blueprints/button.button_C"))
  (Default|InteractCheck _outactors))

(event Input|EnhancedActionEvents|EnhancedInputActionattack
  (params (ActionValue :type Boolean) (ElapsedSeconds :type Float%20%28double-precision%29) (TriggeredSeconds :type Float%20%28double-precision%29) (InputAction :type Input%20Action%20Object%20Reference :default "/Game/Blueprints/character/attack.attack"))
  ;[1 1 1] attack
  (bind _returnvalue (Actor|GetActorOfClass "/Game/Blueprints/character/pickUpItem.pickUpItem_C"))
  (if (Actor|ActorHasTag (Variables|Default|GetActiveItem) "weapon")
    (Default|Attack _returnvalue (Variables|Default|GetdaggerStartRot) (Variables|Default|GetSphere) (Variables|Components|GetCube1))
    (CallFunction|Noise)))

(event Input|EnhancedActionEvents|EnhancedInputActionopenWheel
  (params (ActionValue :type Boolean) (ElapsedSeconds :type Float%20%28double-precision%29) (TriggeredSeconds :type Float%20%28double-precision%29) (InputAction :type Input%20Action%20Object%20Reference :default "/Game/Blueprints/character/openWheel.openWheel"))
  ;[1 1 1] item ui
  (:Triggered
    (bind _foundwidgets (Widget|GetAllWidgetsOfClass "/Game/Blueprints/character/uiBlueprint.uiBlueprint_C" true :!label _label))
    (Default|ToggleRadialVisibility _foundwidgets))
  (:Completed
    (goto _label)))

(event Input|EnhancedActionEvents|EnhancedInputActionscroll
  (params (ActionValue :type Float%20%28double-precision%29) (ElapsedSeconds :type Float%20%28double-precision%29) (TriggeredSeconds :type Float%20%28double-precision%29) (InputAction :type Input%20Action%20Object%20Reference :default "/Game/Blueprints/character/scroll.scroll"))
  ;[1 1 1] item ui
  (bind _foundwidgets (Widget|GetAllWidgetsOfClass "/Game/Blueprints/character/uiBlueprint.uiBlueprint_C" true))
  (Default|ChangeItemIndex _foundwidgets ActionValue))

(event Input|EnhancedActionEvents|EnhancedInputActiondebug
  (params (ActionValue :type Boolean) (ElapsedSeconds :type Float%20%28double-precision%29) (TriggeredSeconds :type Float%20%28double-precision%29) (InputAction :type Input%20Action%20Object%20Reference :default "/Game/Blueprints/character/debug.debug"))
  ;[1 1 1] item ui
  (bind _foundwidgets (Widget|GetAllWidgetsOfClass "/Game/Blueprints/character/uiBlueprint.uiBlueprint_C" true))
  (Default|Debug _foundwidgets))

(event Input|EnhancedActionEvents|EnhancedInputActionlook
  (params (ActionValue :type Vector%202D%20Structure) (ElapsedSeconds :type Float%20%28double-precision%29) (TriggeredSeconds :type Float%20%28double-precision%29) (InputAction :type Input%20Action%20Object%20Reference :default "/Game/Blueprints/character/look.look"))
  (bind _camera (Variables|Default|GetCamera))
  ;[1 1 1] lookin round
  (Pawn|Input|AddControllerYawInput (.x ActionValue))
  (Pawn|Input|AddControllerPitchInput (* (.y ActionValue) -1.0))
  (Physics|Components|PhysicsHandle|SetTargetLocation (Variables|Default|GetPhysicsHandle) (* (Transformation|GetWorldLocation _camera) (* (Math|Vector|GetForwardVector _camera) (Variables|Default|Getline_trace_distance)))))

(event Input|EnhancedActionEvents|EnhancedInputActionmove
  (params (ActionValue :type Vector%202D%20Structure) (ElapsedSeconds :type Float%20%28double-precision%29) (TriggeredSeconds :type Float%20%28double-precision%29) (InputAction :type Input%20Action%20Object%20Reference :default "/Game/Blueprints/character/move.move"))
  (bind _returnvalue (Pawn|GetControlRotation :!class /Script/Engine.Pawn))
  ;[1 1 1] movey ment
  (Pawn|Input|AddMovementInput (Math|Vector|GetRightVector (Math|Rotator|MakeRotator (.roll _returnvalue) 0.0 (.yaw _returnvalue))) (.x ActionValue) false)
  (Pawn|Input|AddMovementInput (Math|Vector|GetForwardVector (Math|Rotator|MakeRotator 0.0 0.0 (.yaw (Pawn|GetControlRotation :!class /Script/Engine.Pawn)))) (.y ActionValue) false))

(event Input|EnhancedActionEvents|EnhancedInputActiondrop
  (params (ActionValue :type Boolean) (ElapsedSeconds :type Float%20%28double-precision%29) (TriggeredSeconds :type Float%20%28double-precision%29) (InputAction :type Input%20Action%20Object%20Reference :default "/Game/Blueprints/character/drop.drop"))
  ;[1 1 1] pick up
  (CallFunction|DropObject))

(event Input|EnhancedActionEvents|EnhancedInputActionsprant
  (params (ActionValue :type Boolean) (ElapsedSeconds :type Float%20%28double-precision%29) (TriggeredSeconds :type Float%20%28double-precision%29) (InputAction :type Input%20Action%20Object%20Reference :default "/Game/Blueprints/character/sprant.sprant"))
  ;[1 1 1] sprinty (disabled)
)

(event Input|EnhancedActionEvents|EnhancedInputActioncrounhc
  (params (ActionValue :type Boolean) (ElapsedSeconds :type Float%20%28double-precision%29) (TriggeredSeconds :type Float%20%28double-precision%29) (InputAction :type Input%20Action%20Object%20Reference :default "/Game/Blueprints/character/crounhc.crounhc"))
  (bind _returnvalue (Transformation|GetActorForwardVector))
  (bind _returnvalue_2 (Game|GetPlayerCharacter 0))
  (bind _slideamount (Variables|Default|GetslideAmount))
  (bind _camera (Variables|Default|GetCamera))
  (bind _camera_2 (Variables|Default|GetCamera))
  (bind _capsulecomponent (Variables|Collision|GetCapsuleComponent))
  (bind _capsulecomponent_2 (Variables|Collision|GetCapsuleComponent))
  (bind _relativescale3d (Variables|/Script/Engine.SceneComponent|GetRelativeScale3D _capsulecomponent_2))
  (bind _relativerotation (Variables|/Script/Engine.SceneComponent|GetRelativeRotation _camera_2))
  (bind _relativerotation_2 (Variables|/Script/Engine.SceneComponent|GetRelativeRotation _camera))
  (bind _relativescale3d_2 (Variables|/Script/Engine.SceneComponent|GetRelativeScale3D _capsulecomponent))
  ;[1 1 1] crounch and slide
  (:Started
    (if (and (Variables|Default|GetisSprinting) (Variables|Default|GetslideReady))
      (Variables|/Script/Engine.CharacterMovementComponent|SetGroundFriction (Variables|Character|GetCharacterMovement) 0.1)
      (Variables|Default|SetslideReady false)
      (Character|LaunchCharacter _returnvalue_2 (Math|Vector|MakeVector (* (.x _returnvalue) _slideamount) (* (.y _returnvalue) _slideamount) 2.0) false false)
      (Variables|/Script/Engine.CharacterMovementComponent|SetGravityScale (Variables|Character|GetCharacterMovement) 2e+03)
      (Variables|Default|SetcameraSlideState (Math|Rotator|MakeRotator 0.0 (.pitch _relativerotation_2) (.yaw _relativerotation_2)))
      (bind (_direction _newtrack_0 _newtrack_1) (Timeline|Timeline_0 PlayFromStart)
        (:Update
          (Transformation|SetRelativeRotation (Variables|Default|GetCamera) (Math|Rotator|MakeRotator (.roll _relativerotation) _newtrack_1 _newtrack_0) false false)
          (Utilities|FlowControl|Delay 0.5)
          (bind (_direction_2 _newtrack_0_2 _newtrack_1_2) (Timeline|Timeline_1 ReverseFromEnd)
            (:Update
              (Transformation|SetRelativeRotation (Variables|Default|GetCamera) (Math|Rotator|MakeRotator (.roll _relativerotation) _newtrack_1_2 _newtrack_0_2) false false)
              (bind _newtrack_0_3 (Timeline|Timeline_3 PlayFromStart)
                (:Update
                  (Transformation|SetRelativeScale3D _capsulecomponent_2 (Math|Vector|MakeVector (.x _relativescale3d) (.y _relativescale3d) _newtrack_0_3))
                  (Utilities|FlowControl|Delay 0.5)
                  (Variables|/Script/Engine.CharacterMovementComponent|SetGravityScale (Variables|Character|GetCharacterMovement) 1.0)
                  (Variables|/Script/Engine.CharacterMovementComponent|SetGroundFriction (Variables|Character|GetCharacterMovement) 8.0)
                  (Variables|Default|SetslideReady true)))))))))
  (:Ongoing
    (Transformation|SetRelativeScale3D _capsulecomponent (Math|Vector|MakeVector (.x _relativescale3d_2) (.y _relativescale3d_2) 0.7))
    (Utilities|FlowControl|DoOnce false :!label _label
      (:Completed
        (Character|LaunchCharacter _returnvalue_2 "0.000000,0.000000,-15.000000" false false))))
  (:Canceled
    (if (Variables|Default|GetslideReady) :!label _label_2
      (bind _newtrack_0_4 (Timeline|Timeline_2 PlayFromStart)
        (:Update
          (Transformation|SetRelativeScale3D _capsulecomponent (Math|Vector|MakeVector (.x _relativescale3d_2) (.y _relativescale3d_2) _newtrack_0_4))
          (goto _label Reset)))))
  (:Completed
    (goto _label_2)))

(event Input|EnhancedActionEvents|EnhancedInputActiongrapple
  (params (ActionValue :type Boolean) (ElapsedSeconds :type Float%20%28double-precision%29) (TriggeredSeconds :type Float%20%28double-precision%29) (InputAction :type Input%20Action%20Object%20Reference :default "/Game/Blueprints/character/grapple.grapple"))
  (bind _returnvalue (Game|GetPlayerCharacter 0))
  (bind _setgrappletarget (Variables|Default|GetsetGrappleTarget))
  (bind _returnvalue_2 (Transformation|GetWorldLocation _setgrappletarget))
  (bind _returnvalue_3 (Transformation|GetActorLocation _returnvalue))
  ;[1 1 1] grpear
  (:Triggered
    (CallFunction|Noise :!label _label)
    (if (not (Variables|Default|GetisGrappling))
      (if (Variables|Default|GetcanGrapple)
        (Variables|Default|SetisGrappling true)
        (Timeline|Timeline_4 Play
          (:Update
            (Physics|AddImpulse (Variables|/Script/Engine.Character|GetCharacterMovement _returnvalue) (Math|Vector|ClampVectorSize (* (Math|Vector|Normalize (- _returnvalue_2 _returnvalue_3)) (Variables|Default|GetgrappleStrength)) 0.0 4e+01) true)
            (if (>= (Math|Vector|Distance(Vector) _returnvalue_3 _returnvalue_2) 4.2e+03)
              (Timeline|Timeline_4 Stop)
              (else
                (Rendering|Debug|DrawDebugArrow :LineStart _returnvalue_3 :LineEnd _returnvalue_2 :Thickness 1.0))))))))
  (:Ongoing
    (goto _label))
  (:Canceled
    (Variables|Default|SetisGrappling false :!label _label_2)
    (Timeline|Timeline_4 Stop))
  (:Completed
    (goto _label_2)))

(event Input|EnhancedActionEvents|EnhancedInputActionreset
  (params (ActionValue :type Boolean) (ElapsedSeconds :type Float%20%28double-precision%29) (TriggeredSeconds :type Float%20%28double-precision%29) (InputAction :type Input%20Action%20Object%20Reference :default "/Game/Blueprints/character/reset.reset"))
  ;[1 1 1] reset position
  (Transformation|SetWorldLocation (Variables|Collision|GetCapsuleComponent) "-2000.000000,-700.000000,100.000000" false false))

(event Input|EnhancedActionEvents|EnhancedInputActionescape
  (params (ActionValue :type Boolean) (ElapsedSeconds :type Float%20%28double-precision%29) (TriggeredSeconds :type Float%20%28double-precision%29) (InputAction :type Input%20Action%20Object%20Reference :default "/Game/Blueprints/character/escape.escape"))
  ;[1 1 1] menu
  (bind _returnvalue (UserInterface|CreateWidget "/Game/levels/prober_jam/ingameMenuUI.ingameMenuUI_C"))
  (Variables|Default|Setmenu _returnvalue)
  (UserInterface|Viewport|AddtoPlayerScreen _returnvalue)
  (Variables|/Script/UMG.Widget|SetVisibility (Variables|Default|GetcrosshairReference) "Hidden"))

(event EventTick
  (params (DeltaSeconds :type Float%20%28single-precision%29))
  (bind _camera (Variables|Default|GetCamera))
  (bind _charactermovement (Variables|Character|GetCharacterMovement))
  (bind _crosshairreference (Variables|Default|GetcrosshairReference))
  (bind _crosshairreference_2 (Variables|Default|GetcrosshairReference))
  (bind _grabicon (Variables|Default|GetgrabIcon))
  (bind _grabicon_2 (Variables|Default|GetgrabIcon))
  (bind _returnvalue (Utilities|IsValid _grabicon_2))
  (bind _returnvalue_2 (Utilities|IsValid _crosshairreference))
  (bind _relativerotation (Variables|/Script/Engine.SceneComponent|GetRelativeRotation _camera))
  ;[1 1 1] wallrunning :)
  (Utilities|FlowControl|FlipFlop
    (:A
      (bind (_outhit _returnvalue_3) (Utilities|WallLineTraceRight 1))
      (bind (_outhit_2 _returnvalue_4) (Utilities|WallLineTraceRight -1))
      (if _returnvalue_3
        (if (Components|ComponentHasTag (.HitComponent (Collision|BreakHitResult _outhit)) "wall")
          (Variables|Default|SetwallSide true)
          (if (not (Pawn|Components|CharacterMovement|IsWalking (Variables|/Script/Engine.Character|GetCharacterMovement (Game|GetPlayerCharacter 0)))) :!label _label
            (Variables|Default|SetisWallrunning true)
            (Variables|/Script/Engine.CharacterMovementComponent|SetGravityScale _charactermovement 0.3)
            (if (not (Variables|Default|Getwallrot))
              (if (Variables|Default|GetwallSide)
                (bind _result (Math|Float|NegateFloat (Math|Float|Absolute(Float) (Variables|Default|GetWallcamOffset)))
                  (:%20%20
                    (Variables|Default|SetWallcamOffset _result)))
                (else
                  (Variables|Default|SetWallcamOffset (Math|Float|Absolute(Float) (Variables|Default|GetWallcamOffset)))))
              (Variables|Default|Setwallrot true)
              (bind _newtrack_0 (Timeline|Timeline ReverseFromEnd)
                (:Update
                  (if (<= (Variables|Default|GetWallcamOffset) 0.0)
                    (Variables|Default|SetspinDir (* _newtrack_0 -1.0))
                    (else
                      (Variables|Default|SetspinDir _newtrack_0)))
                  (Transformation|SetRelativeRotation _camera (Math|Rotator|MakeRotator (Variables|Default|GetspinDir) (.pitch _relativerotation) (.yaw _relativerotation)) false false)))))
          (else
            (Variables|Default|SetisWallrunning false :!label _label_2)
            (Variables|/Script/Engine.CharacterMovementComponent|SetGravityScale _charactermovement 1.0)
            (if (Variables|Default|Getwallrot)
              (Variables|Default|Setwallrot false)
              (Timeline|Timeline PlayFromStart))))
        (elif _returnvalue_4
          (if (Components|ComponentHasTag (.HitComponent (Collision|BreakHitResult _outhit_2)) "wall")
            (Variables|Default|SetwallSide false)
            (goto _label)
            (else
              (goto _label_2)))
          (else
            (goto _label_2)))))
    (:B
      ;[1 1 1] grapple check & crosshair colour change
      (bind _hitcomponent (Utilities|NewMacro))
      (if (Utilities|IsValid _hitcomponent)
        (Variables|Default|SetcrosshairState (Components|ComponentHasTag _hitcomponent "grapple-able"))
        (if (and (Variables|Default|GetcrosshairState) _returnvalue_2)
          (Variables|Default|SetsetGrappleTarget _hitcomponent)
          (Variables|Default|SetcanGrapple true)
          (Appearance|SetColorandOpacity _crosshairreference_2 (Utilities|Struct|MakeLinearColor 0.0 1.0 0.0 1.0) :!class /Script/UMG.Image)
          (GameplayTasks|TaskWaitDelay (stale EventBeginPlay _returnvalue) 1.0
            (:then
              ;;[1 1 1] mantle check & crosshair change
              (bind (_impact_normal_z _hitcomponent_2) (Utilities|NewMacro0 :!label _label_3))
              (if (Utilities|IsValid _hitcomponent_2)
                (if (Math|Boolean|ANDBoolean (not (AI|Components|NavMovement|IsMovingonGround (Variables|Character|GetCharacterMovement))) (Math|Float|InRange(Float) _impact_normal_z 0.85 1.15) (Components|ComponentHasTag _hitcomponent_2 "wall") _returnvalue)
                  (Variables|Default|SetgrabIconState true)
                  (Variables|Default|SetcanMantle true)
                  (Appearance|SetColorandOpacity _grabicon (Utilities|Struct|MakeSlateColor "(R=0.000000,G=1.000000,B=0.003621,A=1.000000)" "UseColor_Specified") :!class /Script/UMG.TextBlock :!label _label_4)
                  (Utilities|FlowControl|Delay 0.5)
                  (Variables|Default|SetcanMantle false)
                  (elif (not (Variables|Default|GetcanMantle))
                    (Variables|Default|SetgrabIconState false :!label _label_5)
                    (if _returnvalue
                      (Appearance|SetColorandOpacity _grabicon (Utilities|Struct|MakeSlateColor "(R=1.000000,G=0.000000,B=1.000000,A=0.000000)" "UseColor_Specified") :!class /Script/UMG.TextBlock))
                    (else
                      (goto _label_4))))
                (else
                  (goto _label_5))))
            (:OnFinish
              (Variables|Default|SetcanGrapple false)))
          (else
            (if (and (not (Variables|Default|GetcanGrapple)) _returnvalue_2) :!label _label_6
              (Appearance|SetColorandOpacity _crosshairreference_2 (Utilities|Struct|MakeLinearColor 1.0 1.0 1.0 1.0) :!class /Script/UMG.Image)
              (goto _label_3))))
        (else
          (goto _label_6))))))

(event EventBeginPlay
  ;[1 1 1] initialization
  (Variables|Default|SetcameraFov (Variables|/Script/Engine.CameraComponent|GetFieldOfView (Variables|Default|GetCamera)))
  (Variables|Default|SetdaggerStartRot (Variables|/Script/Engine.SceneComponent|GetRelativeRotation (Variables|Components|GetCube)))
  (bind _returnvalue (AddComponent|AddGameplayTasksComponent))
  (bind _asplayer_controller (Utilities|Casting|CastToPlayerController (Pawn|GetController)))
  (Utilities|IsValid (PlayerController|LocalPlayerSubsystems|GetEnhancedInputLocalPlayerSubsystem _asplayer_controller)
    (:Is%20Valid
      (Input|AddMappingContext (PlayerController|LocalPlayerSubsystems|GetEnhancedInputLocalPlayerSubsystem _asplayer_controller) "/Game/Blueprints/character/playermovement.playermovement" 0 "(bIgnoreAllPressedKeysUntilRelease=True,bForceImmediately=False,bNotifyUserSettings=False)"))))

(fn ConstructionScript)

(fn StartSprint)

(fn StopSprint)

(fn PickUp
  (bind _camera (Variables|Default|GetCamera))
  (bind _returnvalue (Transformation|GetWorldLocation _camera))
  (bind _foundwidgets (Widget|GetAllWidgetsOfClass "/Game/Blueprints/character/uiBlueprint.uiBlueprint_C" true))
  (if (> 5 (Class|DynamicEntryBoxBase|GetNumEntries (Variables|/Game/Blueprints/character/uiBlueprint.uiBlueprint_C|GetdynamicBox (Utilities|Array|Get(acopy) _foundwidgets))))
    (bind (_outhit _returnvalue_2) (Collision|LineTraceByChannel _returnvalue (+ _returnvalue (* (Math|Vector|GetForwardVector (Transformation|GetWorldRotation _camera)) (* (Variables|Default|Getline_trace_distance) 2.0))) "TraceTypeQuery1" false 0 "None"))
    (if (and _returnvalue_2 (Components|ComponentHasTag (.HitComponent (Collision|BreakHitResult _outhit)) "pickupable"))
      (Physics|SetSimulatePhysics (Actor|GetComponentbyClass (Components|GetOwner (.HitComponent (Collision|BreakHitResult _outhit))) "/Script/Engine.StaticMeshComponent") false)
      (Collision|SetCollisionEnabled (Actor|GetComponentbyClass (Components|GetOwner (.HitComponent (Collision|BreakHitResult _outhit))) "/Script/Engine.StaticMeshComponent") "NoCollision")
      (bind _aspick_up_item (Utilities|Casting|CastTopickUpItem (Components|GetOwner (.HitComponent (Collision|BreakHitResult _outhit)))))
      (bind _foundwidgets_2 (Widget|GetAllWidgetsOfClass "/Game/Blueprints/character/uiBlueprint.uiBlueprint_C" true))
      (Default|AddDude _foundwidgets_2 (Variables|/Game/Blueprints/character/pickUpItem.pickUpItem_C|Geticon _aspick_up_item) (Components|GetOwner (.HitComponent (Collision|BreakHitResult _outhit))))
      (Transformation|AttachComponentToComponent (Components|GetOwner (.HitComponent (Collision|BreakHitResult _outhit))) (Variables|Components|GetCube1) "None" "SnapToTarget" "SnapToTarget" "KeepWorld" true))))

(fn DropObject
  (bind _cube1 (Variables|Components|GetCube1))
  (bind _activeitem (Variables|Default|GetActiveItem))
  (bind _returnvalue (Actor|GetComponentbyClass _activeitem "/Script/Engine.PrimitiveComponent"))
  (if (Utilities|IsValid _activeitem)
    (Rendering|SetActorHiddenInGame _activeitem false)
    (Variables|Default|SetcheckVel (Transformation|GetVelocity (Components|GetOwner _cube1)))
    (Physics|SetSimulatePhysics _returnvalue true)
    (Transformation|DetachFromComponent (Variables|/Script/Engine.Actor|GetRootComponent _activeitem) "KeepWorld" "KeepWorld" "KeepWorld" true)
    (Collision|SetCollisionEnabled (Actor|GetComponentbyClass _activeitem "/Script/Engine.PrimitiveComponent") "QueryAndPhysics")
    (Class|PrimitiveComponent|AddVelocityChangeImpulseatLocation _returnvalue (Variables|Default|GetcheckVel) (Transformation|GetWorldLocation _cube1) "None")
    (bind _foundwidgets (Widget|GetAllWidgetsOfClass "/Game/Blueprints/character/uiBlueprint.uiBlueprint_C" false))
    (Default|RemoveDude _foundwidgets)))
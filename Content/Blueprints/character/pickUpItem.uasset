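; Pick-up item Blueprint that provides a melee attack against Big_guy_homie's weak points.
; The attack event, gated to actors without the "weapon" tag, plays a timeline that swings the passed component by scaling the dagger's starting roll.
; Each update tests the passed sphere against the first found boss's weak points, setting AttackedPoint and Attacked on overlap.
; The MadeVulnerable check has no effect, as both branches continue identically.
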(event Custom|attack
  (params (daggerStartRot :type Rotator) (shphere :type Primitive%20Component%20Object%20Reference) (cubeeb :type Scene%20Component%20Object%20Reference))
  ;[1 1 1] attack
  (if (not (Actor|ActorHasTag self "weapon"))
    (bind _newtrack_0 (Timeline|Timeline PlayFromStart)
      (:Update
        (Transformation|SetRelativeRotation cubeeb (Math|Rotator|MakeRotator (* _newtrack_0 (.roll daggerStartRot)) (.pitch daggerStartRot) (.yaw daggerStartRot)) false false)
        (bind _returnvalue (Actor|GetActorOfClass "/Game/Blueprints/big_guy/big_guy_homie.big_guy_homie_C"))
        (for _array_element (Variables|/Game/Blueprints/big_guy/big_guy_homie.big_guy_homie_C|GetfullWeakPoints _returnvalue)
          (if (Class|PrimitiveComponent|IsOverlappingComponent shphere _array_element)
            (Variables|/Game/Blueprints/big_guy/big_guy_homie.big_guy_homie_C|SetattackedPoint _returnvalue _array_element)
            (if (Variables|/Game/Blueprints/big_guy/big_guy_homie.big_guy_homie_C|GetmadeVulnerable _returnvalue)
              _
              (else
                _))
            (Variables|/Game/Blueprints/big_guy/big_guy_homie.big_guy_homie_C|Setattacked _returnvalue true)))))))

(event EventBeginPlay)

(event Collision|EventActorBeginOverlap
  (params (OtherActor :type Actor%20Object%20Reference)))

(event EventTick
  (params (DeltaSeconds :type Float%20%28single-precision%29)))

(fn ConstructionScript)